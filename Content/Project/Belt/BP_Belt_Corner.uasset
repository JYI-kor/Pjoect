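; Corner conveyor belt piece, apparently a child of a base belt, that supplies a curved movement direction for a target location.
; GetMoveVector treats the Arrow component as the pivot, using the right vector of the look-at rotation toward it as the main tangential push.
; A small radial term pulls inward beyond a fixed radius and pushes outward otherwise, steering targets onto a circular path.
; Event graph is unused; construction only calls the parent.
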(event EventBeginPlay)

(event Collision|EventActorBeginOverlap
  (params (OtherActor :type Actor%20Object%20Reference)))

(event EventTick
  (params (DeltaSeconds :type Float%20%28single-precision%29)))

(fn ConstructionScript
  (|CallParentFunction))

(fn GetMoveVector
  (params (Target%20Location :type Vector :default "0, 0, 0"))
  (bind _arrow (Variables|Default|GetArrow))
  (bind _returnvalue (Transformation|GetWorldLocation _arrow))
  (bind _returnvalue_2 (Math|Rotator|FindLookatRotation Target%20Location _returnvalue))
  (bind _returnvalue_3 (Math|Vector|GetRightVector _returnvalue_2))
  (bind _returnvalue_4 (Math|Vector|GetForwardVector _returnvalue_2))
  (bind _returnvalue_5 (* _returnvalue_3 2.0))
  (if (> (Math|Vector|Distance(Vector) Target%20Location _returnvalue) 3.3e+02)
    (return (+ (* _returnvalue_4 0.1) _returnvalue_5))
    (else
      (return (+ (* _returnvalue_4 -0.1) _returnvalue_5)))))